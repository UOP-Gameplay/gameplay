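; In-world main menu actor for Retail Therapy, showing a logo with Play and Quit screens.
; A timeline bounces the logo, while ButtonInput cycles the selection and recolours the screens through dynamic material instances.
; AcceptButton either starts the game via RetailTherapy_GS or quits.
; The game state's start and end events hide and restore the menu meshes.
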(event Custom|Game%20End
  (Rendering|SetVisibility (Variables|Default|GetLogo) true false))

(event Custom|Game%20Start
  (Rendering|SetVisibility (Variables|Default|GetLogo) false false))

(event EventBeginPlay
  (bind _asretail_therapy_gs (Utilities|Casting|CastToRetailTherapy_GS (Game|GetGameState)))
  (EventDispatchers|BindEventtoGameStarted _asretail_therapy_gs (delegate Custom|Game%20Start))
  (EventDispatchers|BindEventtoGameEnd _asretail_therapy_gs (delegate Custom|Game%20End))
  (Components|Timeline|PlayfromStart (Variables|Default|GetLogoBounce))
  (bind _returnvalue (Rendering|Material|CreateDynamicMaterialInstance (Variables|Default|GetScreen_Play) 0 "/Game/Menus/Assets/MI_Flat_Play.MI_Flat_Play" "None" :!class /Script/Engine.PrimitiveComponent))
  (Variables|Default|SetPlay%20Material _returnvalue)
  (bind _returnvalue_2 (Rendering|Material|CreateDynamicMaterialInstance (Variables|Default|GetScreen_Quit) 0 "/Game/Menus/Assets/MI_Flat_Quit.MI_Flat_Quit" "None" :!class /Script/Engine.PrimitiveComponent))
  (Variables|Default|SetQuit%20Material _returnvalue_2)
  (Rendering|Material|SetVectorParameterValue (Variables|Default|GetPlay%20Material) "Colour" (Variables|Default|GetSelected%20Colour) :!class /Script/Engine.MaterialInstanceDynamic)
  (Rendering|Material|SetVectorParameterValue (Variables|Default|GetQuit%20Material) "Colour" (Variables|Default|GetDeselected%20Colour) :!class /Script/Engine.MaterialInstanceDynamic))

(event Collision|EventActorBeginOverlap
  (params (OtherActor :type Actor%20Object%20Reference)))

(event EventTick
  (params (DeltaSeconds :type Float%20%28single-precision%29)))

(fn ConstructionScript)

(fn ButtonInput
  (params (Down :type Boolean))
  (bind _selected_colour (Variables|Default|GetSelected%20Colour))
  (bind _deselected_colour (Variables|Default|GetDeselected%20Colour))
  (if Down
    (Variables|Default|SetIndex (+ (Variables|Default|GetIndex) 1))
    (if (> (Variables|Default|GetIndex) 1)
      (Variables|Default|SetIndex 0))
    (elif (== (Variables|Default|GetIndex) 0)
      (Variables|Default|SetIndex 1)
      (else
        (Variables|Default|SetIndex (- (Variables|Default|GetIndex) 1)))))
  (switch int (Math|Conversions|ToInteger(Byte) (Variables|Default|GetIndex))
    (:0
      (Rendering|Material|SetVectorParameterValue (Variables|Default|GetPlay%20Material) "Colour" _selected_colour :!class /Script/Engine.MaterialInstanceDynamic)
      (Rendering|Material|SetVectorParameterValue (Variables|Default|GetQuit%20Material) "Colour" _deselected_colour :!class /Script/Engine.MaterialInstanceDynamic))
    (:1
      (Rendering|Material|SetVectorParameterValue (Variables|Default|GetPlay%20Material) "Colour" _deselected_colour :!class /Script/Engine.MaterialInstanceDynamic)
      (Rendering|Material|SetVectorParameterValue (Variables|Default|GetQuit%20Material) "Colour" _selected_colour :!class /Script/Engine.MaterialInstanceDynamic))))

(fn AcceptButton
  (switch int (Math|Conversions|ToInteger(Byte) (Variables|Default|GetIndex))
    (:0
      (bind _asretail_therapy_gs (Utilities|Casting|CastToRetailTherapy_GS (Game|GetGameState)))
      (Default|StartGame _asretail_therapy_gs))
    (:1
      (Game|QuitGame 0 "Quit" false))))