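; Title screen actor that animates an expanding sphere followed by an opacity fade on the main menu logo.
; BeginPlay sets a short delay timer, presumably to start PushSphere, though its bound event is not shown.
; PushSphere scales the sphere up through a timeline, then calls FadeText on completion.
; FadeText creates a dynamic material instance on the logo mesh and drives its Opacity parameter with a second timeline.
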(event Custom|PushSphere
  (bind _alpha (Timeline|SphereScale Play)
    (:Update
      (Transformation|SetWorldScale3D (Variables|Default|GetSphere) (Math|Vector|Lerp(Vector) "25.000000,25.000000,25.000000" "250.000000,250.000000,250.000000" _alpha)))
    (:Finished
      (CallFunction|FadeText))))

(event Custom|FadeText
  (bind _returnvalue (Rendering|Material|CreateDynamicMaterialInstance (Variables|Default|GetStaticMesh) 0 "/Game/Menus/Assets/M_Mainmenu_Logo.M_Mainmenu_Logo" "None" :!class /Script/Engine.PrimitiveComponent))
  (bind _newtrack_0 (Timeline|TextFade Play)
    (:Update
      (Rendering|Material|SetScalarParameterValue _returnvalue "Opacity" _newtrack_0 :!class /Script/Engine.MaterialInstanceDynamic))))

(event EventBeginPlay
  (Utilities|Time|SetTimerbyEvent (EventDispatchers|CreateEvent :!event Custom|PushSphere) 3.0))

(event Collision|EventActorBeginOverlap
  (params (OtherActor :type Actor%20Object%20Reference)))

(event EventTick
  (params (DeltaSeconds :type Float%20%28single-precision%29)))

(fn ConstructionScript)